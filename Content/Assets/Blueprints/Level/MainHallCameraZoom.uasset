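; Trigger volume for the main hall that zooms the player's camera out on entry and back in on exit.
; Box overlaps with the cached Teardevil character set a Transition state to Expand or Shrink.
; Tick uses FInterpTo to ease the SpringArm's target length toward the far or near distance.
; Near either target, it clears the state and sets the arm length to zero.
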(event `self.ReceiveBeginPlay`
  (bind _asteardevil_character_bp (cast `/Game/Assets/Blueprints/Characters/TeardevilCharacterBP` (`GameplayStatics.GetPlayerPawn` 0)))
  (set `self.Character` _asteardevil_character_bp))

(event `self.ReceiveTick`
  (params (DeltaSeconds :type "Float (single-precision)"))
  (bind _transition (`self.Transition`))
  (bind _springarm (`/Game/Assets/Blueprints/Characters/TeardevilCharacterBP.SpringArm` (`self.Character`)))
  (bind _springarm_2 (`/Game/Assets/Blueprints/Characters/TeardevilCharacterBP.SpringArm` (`self.Character`)))
  (bind _springarm_3 (`/Game/Assets/Blueprints/Characters/TeardevilCharacterBP.SpringArm` (`self.Character`)))
  (if (== _transition "Expand")
    (bind _output_get (set `SpringArmComponent.TargetArmLength` (`KismetMathLibrary.FInterpTo` (`SpringArmComponent.TargetArmLength` _springarm_2) 2000.0 (`GameplayStatics.GetWorldDeltaSeconds`) 1.0) _springarm_2))
    (if (>= _output_get 1998.0)
      (set `self.Transition` "None")
      (set `SpringArmComponent.TargetArmLength` 0.0 _springarm))
    (elif (== _transition "Shrink")
      (bind _output_get_2 (set `SpringArmComponent.TargetArmLength` (`KismetMathLibrary.FInterpTo` (`SpringArmComponent.TargetArmLength` _springarm_3) 800.0 (`GameplayStatics.GetWorldDeltaSeconds`) 1.0) _springarm_3))
      (if (<= _output_get_2 802.0)
        (set `self.Transition` "None")
        (set `SpringArmComponent.TargetArmLength` 0.0 _springarm)))))

(event `self.Box.OnComponentBeginOverlap`
  (params (OverlappedComponent :type "PrimitiveComponent Object Reference") (OtherActor :type "Actor Object Reference") (OtherComp :type "PrimitiveComponent Object Reference") (OtherBodyIndex :type Integer) (bFromSweep :type Boolean) (SweepResult :type "HitResult Structure (by ref)"))
  (if (== OtherActor (`self.Character`))
    (set `self.Transition` "Expand")))

(event `self.Box.OnComponentEndOverlap`
  (params (OverlappedComponent :type "PrimitiveComponent Object Reference") (OtherActor :type "Actor Object Reference") (OtherComp :type "PrimitiveComponent Object Reference") (OtherBodyIndex :type Integer))
  (if (== (`self.Character`) OtherActor)
    (set `self.Transition` "Shrink")))

(fn `UserConstructionScript`)