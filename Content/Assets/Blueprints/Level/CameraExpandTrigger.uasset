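; A level trigger actor that zooms the Teardevil player's camera out while the character overlaps it and back in when it leaves.
; BeginPlay caches the player character and stores its starting spring arm length as the shrink value.
; Overlap begin and end set an Expand or Shrink transition state.
; Tick interpolates the spring arm length toward that target with FInterpTo, snapping and clearing the state once close.
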(event `self.ReceiveBeginPlay`
  (bind _asteardevil_character_bp (cast `/Game/Assets/Blueprints/Characters/TeardevilCharacterBP` (`GameplayStatics.GetPlayerPawn` 0)))
  (bind _output_get (set `self.Character` _asteardevil_character_bp))
  (set `self.ShrinkValue` (`SpringArmComponent.TargetArmLength` (`/Game/Assets/Blueprints/Characters/TeardevilCharacterBP.SpringArm` _output_get))))

(event `self.ReceiveTick`
  (params (DeltaSeconds :type "Float (single-precision)"))
  (bind _transition (`self.Transition`))
  (bind _springarm (`/Game/Assets/Blueprints/Characters/TeardevilCharacterBP.SpringArm` (`self.Character`)))
  (bind _springarm_2 (`/Game/Assets/Blueprints/Characters/TeardevilCharacterBP.SpringArm` (`self.Character`)))
  (if (== _transition "Expand")
    (bind _output_get (set `SpringArmComponent.TargetArmLength` (`KismetMathLibrary.FInterpTo` (`SpringArmComponent.TargetArmLength` _springarm) (`self.ExpandValue`) (`GameplayStatics.GetWorldDeltaSeconds`) 1.0) _springarm))
    (if (>= _output_get (- (`self.ExpandValue`) 2.0))
      (set `self.Transition` "None")
      (set `SpringArmComponent.TargetArmLength` (`self.ExpandValue`) (`/Game/Assets/Blueprints/Characters/TeardevilCharacterBP.SpringArm` (`self.Character`))))
    (elif (== _transition "Shrink")
      (bind _output_get_2 (set `SpringArmComponent.TargetArmLength` (`KismetMathLibrary.FInterpTo` (`SpringArmComponent.TargetArmLength` _springarm_2) (`self.ShrinkValue`) (`GameplayStatics.GetWorldDeltaSeconds`) 1.0) _springarm_2))
      (if (<= _output_get_2 (+ (`self.ShrinkValue`) 2.0))
        (set `self.Transition` "None")
        (set `SpringArmComponent.TargetArmLength` (`self.ShrinkValue`) (`/Game/Assets/Blueprints/Characters/TeardevilCharacterBP.SpringArm` (`self.Character`)))))))

(event `self.ReceiveActorBeginOverlap`
  (params (OtherActor :type "Actor Object Reference"))
  (if (== OtherActor (`self.Character`))
    (set `self.Transition` "Expand")))

(event `self.ReceiveActorEndOverlap`
  (params (OtherActor :type "Actor Object Reference"))
  (if (== (`self.Character`) OtherActor)
    (set `self.Transition` "Shrink")))

(fn `UserConstructionScript`)