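; Game instance Blueprint that holds the score and elapsed play time and toggles the score UI.
; Score events wrap functions that add, clear or set the score, with a getter for reading it.
; A timer event starts a looping one-second TimeCount that rolls seconds into minutes, read through GetTimeCount.
; ShowScoreUI creates a UI_Score widget and adds it to the viewport, or removes the stored one.
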(event `ShowScoreUI`
  (params (value :type Boolean))
  (bind _scorewidget (`self.ScoreWidget`))
  ;[1 1 1] Toggle Score UI
  (if value
    (bind _returnvalue (`|CreateWidget` "/Game/UI/Score/UI_Score.UI_Score_C" (`GameplayStatics.GetPlayerController` 0)))
    (bind _output_get (set `self.ScoreWidget` _returnvalue))
    (`UserWidget.AddToViewport` _output_get 0)
    (else
      (`/Engine/EditorBlueprintResources/StandardMacros.IsValid` _scorewidget
        (:`Is Valid`
          (`Widget.RemoveFromParent` _scorewidget))))))

(event `StartTimerEvent`
  (`KismetSystemLibrary.K2_SetTimer` null "TimeCount" 1.0 true))

(event `AddScoreEvent`
  (params (Score :type Integer))
  ;[1 0.4844 0.4844] Score Events
  (`self.AddScore` Score))

(event `ClearScoreEvent`
  ;[1 0.4844 0.4844] Score Events
  (`self.ClearScore`))

(event `SetScoreEvent`
  (params (Score :type Integer))
  ;[1 0.4844 0.4844] Score Events
  (`self.SetScore` Score))

(fn `AddScore`
  (params (score :type Integer))
  (set `self.Score` (+ (`self.Score`) score)))

(fn `ClearScore`
  (set `self.Score` 0))

(fn `GetScore`
  (returns (score :type Integer))
  (return (`self.Score`)))

(fn `GetTimeCount`
  (returns (Min :type Integer) (Sec :type Integer))
  (return (`self.Min`) (`self.Sec`)))

(fn `SetScore`
  (params (NewScore :type Integer))
  (set `self.Score` NewScore))

(fn `TimeCount`
  (`/Engine/EditorBlueprintResources/StandardMacros.IncrementInt` (`self.Sec`)
    (:`  `
      (if (== (`self.Sec`) 60)
        (set `self.Sec` 0)
        (`/Engine/EditorBlueprintResources/StandardMacros.IncrementInt` (`self.Min`))))))