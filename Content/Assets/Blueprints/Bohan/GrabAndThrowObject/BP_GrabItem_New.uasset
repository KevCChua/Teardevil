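; BP_GrabItem_New is a grabbable, throwable item with a destructible component and a radial force.
; On BeginPlay it optionally turns on physics simulation for the destructible component.
; The construction script removes the radial force unless the item should break its container on grab.
; Mesh hits on an EnemyCharacter at high velocity only print a debug hit message.
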(event `self.ReceiveBeginPlay`
  (bind _pysicsbydefualt (`self.PysicsByDefualt`))
  (if _pysicsbydefualt
    (`PrimitiveComponent.SetSimulatePhysics` (`self.DestructibleComponent`) _pysicsbydefualt)))

(event `self.StaticMesh.OnComponentHit`
  (params (HitComponent :type "PrimitiveComponent Object Reference") (OtherActor :type "Actor Object Reference") (OtherComp :type "PrimitiveComponent Object Reference") (NormalImpulse :type "Vector Structure") (Hit :type "HitResult Structure (by ref)"))
  (if (>= (`KismetMathLibrary.VSize` (`self.GetVelocity`)) 500.0)
    (cast `EnemyCharacter` OtherActor)
    (`KismetSystemLibrary.PrintString` "hit" true true (struct :`G` 0.66 :`B` 1.0 :`A` 1.0) 5.0)))

(fn `UserConstructionScript`
  ;[1 1 1] If should break Container
  (if (not (`self.ShouldBreakContainerOnGrab`))
    (`ActorComponent.K2_DestroyComponent` (`self.RadialForce`))))