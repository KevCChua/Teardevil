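; BP_ActionBubble is a short-lived action bubble that pops up at a spawn point with a randomized look, position and size.
; Construction picks a material set by bubble type (enemy, destructible or easter egg), randomly offsets the actor in XY, and applies a random or start material to Pow.
; BeginPlay chooses a random X/Y end size, scales toward it along a timeline curve, and destroys the actor after its lifetime.
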(event `self.ReceiveBeginPlay`
  ;[1 1 1] Init the end size base on its Start size
  (set `self.MaxX` (`KismetMathLibrary.RandomFloatInRange` 1.0 (`self.SizeX`)))
  (set `self.MaxY` (`KismetMathLibrary.RandomFloatInRange` 0.5 (`self.SizeY`)))
  ;[1 1 1] Animation for the bubble
  (bind (_direction _pop) (`Timeline|Timeline_0`)
    (:`Update`
      (`self.SetActorScale3D` (`KismetMathLibrary.VLerp` (`self.StartSize`) (`KismetMathLibrary.MakeVector` (`self.MaxX`) (`self.MaxY`) 1.0) _pop))
      ;[1 1 1] Kill the bubble after lifetime
      (`KismetSystemLibrary.Delay` (`self.LifeTime`))
      (`self.K2_DestroyActor`))))

(fn `InitBubbleType`
  (switch `/Game/Assets/Blueprints/Bohan/ActionBubbles/E_BubbleType` (`self.BubbleType`)
    (:`NewEnumerator0`
      (set `self.UsingMatarials` (`self.OnEnemyDefaultMaterials`)))
    (:`NewEnumerator1`
      (set `self.UsingMatarials` (`self.OnDestructibleDefaultMaterials`)))
    (:`NewEnumerator3`
      (set `self.UsingMatarials` (`self.OnEasterEggDefaultMaterials`)))))

(fn `InitRandomMaterial`
  (bind _usingmatarials (`self.UsingMatarials`))
  ;[1 1 1] Assign a random material to the bubble
  (`PrimitiveComponent.SetMaterial` (`self.Pow`) 0 (`|GetArrayItem` _usingmatarials (`KismetMathLibrary.RandomIntegerInRange` 0 (- (`KismetArrayLibrary.Array_Length` _usingmatarials) 1)))))

(fn `InitRandomPosition`
  (bind (_randomspawnarea_x _randomspawnarea_y) (`KismetMathLibrary.BreakVector` (`self.RandomSpawnArea`)))
  ;[1 1 1] Add random spawn position base on spawn point
  (bind _result (`/Engine/EditorBlueprintResources/StandardMacros.NegateFloat` _randomspawnarea_x)
    (:`  `
      (bind _result_2 (`/Engine/EditorBlueprintResources/StandardMacros.NegateFloat` _randomspawnarea_y)
        (:`  `
          (`self.K2_AddActorWorldOffset` (`KismetMathLibrary.MakeVector` (`KismetMathLibrary.RandomFloatInRange` _result _randomspawnarea_x) (`KismetMathLibrary.RandomFloatInRange` _result_2 _randomspawnarea_y)) false true))))))

(fn `UserConstructionScript`
  (`self.InitBubbleType`)
  (`self.InitRandomPosition`)
  (if (`self.ShouldUseRandomMatarial`)
    (`self.InitRandomMaterial`)
    (else
      ;[1 1 1] Set Material to the Start Material
      (`PrimitiveComponent.SetMaterial` (`self.Pow`) 0 (`self.StartMaterial`)))))