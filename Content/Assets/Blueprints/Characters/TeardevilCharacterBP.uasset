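; Player character Blueprint for Teardevil that grabs a random nearby item and throws it, adding score on button release.
; Large items stop movement and are spun with right-stick rotation to build throw power.
; Each tick, a velocity-led camera respects traced BP_CameraBound limits, while camera-to-player traces swap tagged blocking meshes' materials and restore them when clear.
; It also has a timeline-faded slow-motion event, debug printing and disconnected stick-direction punch test logic.
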(event `CameraEvents`
  ;[1 0.2083 0.2083] Camera, Aim
  (`self.CheckForCamBound`)
  (`self.SmoothCamera`)
  (`self.RedRayCamera`))

(event `self.ReceiveBeginPlay`
  ;[1 1 1] Begin Play
  (`self.InitEverything`))

(event `Do Slow Motion`
  ;[1 0.2083 0.2083] Camera, Aim
  (bind (_direction _alpha) (`Timeline|SlowFade` :!via `PlayFromStart`)
    (:`Update`
      (`self.SlowMotion` _alpha))))

(event `self.ReceiveTick`
  (params (DeltaSeconds :type "Float (single-precision)"))
  ;[0.4536 1 0.3115] Tick
  (`self.CameraEvents`)
  (`self.ControlEvents`)
  (for _array_element (`self.DirectionArray`)
    (set `self.TestString` (`KismetStringLibrary.Concat_StrStr` (`self.TestString`) (`KismetStringLibrary.Conv_IntToString` _array_element))))
  (`KismetSystemLibrary.PrintString` (`self.TestString`) true true (struct :`G` 0.66 :`B` 1.0 :`A` 1.0) 0.0)
  (set `self.TestString` ""))

(event `ControlEvents`
  ;[1 0.2083 0.2083] Camera, Aim
  (`self.LargeObjectThrowing`))

(event `self.GrabItemCollider.OnComponentBeginOverlap`
  (params (OverlappedComponent :type "PrimitiveComponent Object Reference") (OtherActor :type "Actor Object Reference") (OtherComp :type "PrimitiveComponent Object Reference") (OtherBodyIndex :type Integer) (bFromSweep :type Boolean) (SweepResult :type "HitResult Structure (by ref)"))
  ;[0.4016 0.3133 1] Events
  ;;[1 1 1] Create Object Array When Enter Collision and Exit
  (bind _asbp_grab_item (cast `/Game/Assets/Blueprints/Bohan/GrabAndThrowObject/BP_GrabItem` OtherActor))
  (`KismetArrayLibrary.Array_Add` (`self.ItemsInRange`) _asbp_grab_item))

(event `InputAction|GrabAndThrow`
  (params (Key :type "Key Structure"))
  ;[0.4016 0.3133 1] Events
  ;;[1 1 1] Press Grab And Release Grab
  (:`Pressed`
    (`self.GrabObject`))
  (:`Released`
    (`self.ThrowObject`)
    (`/Game/Assets/Blueprints/IGame_Instance.AddScore` (`self.Game`) 30)))

(event `self.GrabItemCollider.OnComponentEndOverlap`
  (params (OverlappedComponent :type "PrimitiveComponent Object Reference") (OtherActor :type "Actor Object Reference") (OtherComp :type "PrimitiveComponent Object Reference") (OtherBodyIndex :type Integer))
  ;[0.4016 0.3133 1] Events
  ;;[1 1 1] Create Object Array When Enter Collision and Exit
  (bind _asbp_grab_item (cast `/Game/Assets/Blueprints/Bohan/GrabAndThrowObject/BP_GrabItem` OtherActor))
  (`KismetArrayLibrary.Array_RemoveItem` (`self.ItemsInRange`) _asbp_grab_item))

(fn `CheckForCamBound`
  (bind _returnvalue (+ (`self.K2_GetActorLocation`) (/ (`self.GetVelocity`) 6.0)))
  (`|ExecutionSequence`
    (:`then_0`
      (bind _outhit (`KismetSystemLibrary.LineTraceSingle` :`Start` _returnvalue :`End` (+ _returnvalue (`KismetMathLibrary.MakeVector` (`self.CameraBoundCheckLength`))) :`TraceChannel` "TraceTypeQuery1" :`DrawDebugType` (`self.TraceDebug`) :`DrawTime` 0.1))
      (cast `/Game/Assets/Blueprints/Bohan/CameraBound/BP_CameraBound` (`.HitActor` (`GameplayStatics.BreakHitResult` _outhit)))
      (set `self.IsCameraXFree` false))
    (:`then_1`
      (bind _outhit_2 (`KismetSystemLibrary.LineTraceSingle` :`Start` _returnvalue :`End` (+ _returnvalue (`KismetMathLibrary.MakeVector` (* (`self.CameraBoundCheckLength`) -1.0))) :`TraceChannel` "TraceTypeQuery1" :`DrawDebugType` (`self.TraceDebug`) :`TraceColor` (struct :`R` 1.0 :`G` 0.75 :`A` 1.0) :`DrawTime` 0.1))
      (cast `/Game/Assets/Blueprints/Bohan/CameraBound/BP_CameraBound` (`.HitActor` (`GameplayStatics.BreakHitResult` _outhit_2)))
      (set `self.IsCameraXFree` false))
    (:`then_2`
      (bind _outhit_3 (`KismetSystemLibrary.LineTraceSingle` :`Start` _returnvalue :`End` (+ _returnvalue (`KismetMathLibrary.MakeVector` 0.0 (`self.CameraBoundCheckLength`))) :`TraceChannel` "TraceTypeQuery1" :`DrawDebugType` (`self.TraceDebug`) :`TraceColor` (struct :`R` 0.033035 :`B` 1.0 :`A` 1.0) :`DrawTime` 0.1))
      (cast `/Game/Assets/Blueprints/Bohan/CameraBound/BP_CameraBound` (`.HitActor` (`GameplayStatics.BreakHitResult` _outhit_3)))
      (set `self.IsCameraYFree` false))
    (:`then_3`
      (bind _outhit_4 (`KismetSystemLibrary.LineTraceSingle` :`Start` _returnvalue :`End` (+ _returnvalue (`KismetMathLibrary.MakeVector` 0.0 (* (`self.CameraBoundCheckLength`) -1.0))) :`TraceChannel` "TraceTypeQuery1" :`DrawDebugType` (`self.TraceDebug`) :`TraceColor` (struct :`G` 0.697917 :`B` 0.066028 :`A` 1.0) :`DrawTime` 0.1))
      (cast `/Game/Assets/Blueprints/Bohan/CameraBound/BP_CameraBound` (`.HitActor` (`GameplayStatics.BreakHitResult` _outhit_4)))
      (set `self.IsCameraYFree` false))))

(fn `GrabObject`
  (bind _returnvalue (`KismetArrayLibrary.Array_Length` (`self.ItemsInRange`)))
  (bind _staticmesh (`/Game/Assets/Blueprints/Bohan/GrabAndThrowObject/BP_GrabItem.StaticMesh` (`self.HoldingItem`)))
  ;[1 1 1] CheckArray Not Empty, Pick A Random Object In Range
  (if (!= _returnvalue 0)
    (set `self.HoldingItem` (`|GetArrayItem` (`self.ItemsInRange`) (`KismetMathLibrary.RandomIntegerInRange` 0 (- _returnvalue 1))))
    ;[1 1 1] Attach Object To Hand, Set Physics Off
    (`PrimitiveComponent.SetSimulatePhysics` _staticmesh false)
    (`PrimitiveComponent.SetCollisionEnabled` _staticmesh "NoCollision")
    (`self.K2_AttachToComponent` (`self.HoldingItem`) (`self.Mesh`) "hand_rSocket" "SnapToTarget" "SnapToTarget" "KeepRelative" true)
    (set `self.IsHoldingItem` true)
    (if (`/Game/Assets/Blueprints/Bohan/GrabAndThrowObject/BP_GrabItem.IsLargeObject` (`self.HoldingItem`))
      (set `CharacterMovementComponent.MaxWalkSpeed` 0.0 (`self.CharacterMovement`))
      (set `CharacterMovementComponent.JumpZVelocity` 0.0 (`self.CharacterMovement`))
      (set `self.bIsHolding` true))))

(fn `InitEverything`
  ;[1 1 1] Enable Player Input
  (`self.EnableInput` (`GameplayStatics.GetPlayerController` 0) null)
  ;[1 1 1] Init game instance
  (bind _asigame_instance (cast `/Game/Assets/Blueprints/IGame_Instance` (`GameplayStatics.GetGameInstance`)))
  (set `self.Game` _asigame_instance))

(fn `LargeObjectThrowing`
  (bind _maxspinspeed (`self.MaxSpinSpeed`))
  (bind _maxspinspeed_2 (`self.MaxSpinSpeed`))
  (bind _returnvalue (`KismetMathLibrary.DegAtan2` (`self.RightStickY`) (`self.RightStickX`)))
  ;[1 1 1] Checking if player is holding a large object
  (if (`self.IsHoldingItem`)
    (`/Engine/EditorBlueprintResources/StandardMacros.IsValid` (`self.HoldingItem`)
      (:`Is Valid`
        (if (`/Game/Assets/Blueprints/Bohan/GrabAndThrowObject/BP_GrabItem.IsLargeObject` (`self.HoldingItem`))
          (`|ExecutionSequence`
            (:`then_0`
              ;[0.3248 0.4161 1] This is the easiest way i can think of to get player spin gradually
              ;;[1 1 1] Increse Spin speed
              (if (== (- (`KismetMathLibrary.DegAtan2` (`self.RightStickY`) (`self.RightStickX`)) (`self.LastDegree`)) 90.0)
                (set `self.SpinSpeed` (`KismetMathLibrary.FClamp` (+ (`self.SpinSpeed`) (* (`self.SpinAdd`) (`GameplayStatics.GetWorldDeltaSeconds`))) (* _maxspinspeed_2 -1.0) _maxspinspeed_2))
                (elif (== (- (`KismetMathLibrary.DegAtan2` (`self.RightStickY`) (`self.RightStickX`)) (`self.LastDegree`)) -90.0)
                  (set `self.SpinSpeed` (`KismetMathLibrary.FClamp` (+ (`self.SpinSpeed`) (* (* (`self.SpinAdd`) -1.0) (`GameplayStatics.GetWorldDeltaSeconds`))) (* _maxspinspeed -1.0) _maxspinspeed)))))
            (:`then_1`
              ;;[1 1 1] Checking for UDLR
              (if (or (== _returnvalue 180.0) (== _returnvalue 90.0) (== _returnvalue 0.0) (== _returnvalue -90.0))
                (if (!= (- (`KismetMathLibrary.DegAtan2` (`self.RightStickY`) (`self.RightStickX`)) (`self.LastDegree`)) 0.0)
                  (set `self.LastDegree` (`KismetMathLibrary.DegAtan2` (`self.RightStickY`) (`self.RightStickX`))))))
            (:`then_2`
              ;;[1 1 1] Applying Spin Speed and power
              (`self.K2_AddActorWorldRotation` (`KismetMathLibrary.MakeRotator` 0.0 0.0 (`self.SpinSpeed`)))
              (set `self.SpinPower` (`KismetMathLibrary.FClamp` (* (`KismetMathLibrary.Abs` (`self.SpinSpeed`)) (`self.SpinMuiltiplyer`)) 20000.0 (`self.ThrowPower`))))))))))

(fn `RedRayCamera`
  (bind _detectedcomponents (`self.DetectedComponents`))
  (bind _meshmatmap (`self.MeshMatMap`))
  (`|ExecutionSequence`
    (:`then_0`
      (bind _outhits (`KismetSystemLibrary.LineTraceMulti` :`Start` (`SceneComponent.K2_GetComponentLocation` (`self.Camera`)) :`End` (`self.K2_GetActorLocation`) :`TraceChannel` "TraceTypeQuery3" :`DrawDebugType` (`self.TraceDebug`) :`TraceColor` (struct :`R` 1.0 :`G` 1.0 :`B` 1.0 :`A` 1.0) :`DrawTime` 0.1))
      (for _array_element _outhits
        (`self.DoTags` (`ActorComponent.ComponentTags` (`.HitComponent` (`GameplayStatics.BreakHitResult` _array_element)))
          (:`HasTag`
            (bind _asstatic_mesh_component (cast `StaticMeshComponent` (`.HitComponent` (`GameplayStatics.BreakHitResult` _array_element))))
            (set `self.BlockingMesh` _asstatic_mesh_component)
            (if (!= (`PrimitiveComponent.GetMaterial` (`self.BlockingMesh`) 0) (`self.UsingMat`))
              (`KismetArrayLibrary.Array_Add` (`self.DetectedComponents`) (`self.BlockingMesh`))
              (`BlueprintMapLibrary.Map_Add` (`self.MeshMatMap`) (`self.BlockingMesh`) (`PrimitiveComponent.GetMaterial` (`self.BlockingMesh`) 0))
              (`PrimitiveComponent.SetMaterial` (`self.BlockingMesh`) 0 (`self.UsingMat`)))))))
    (:`then_1`
      (if (== (`KismetArrayLibrary.Array_Length` _outhits) 0)
        (for _array_element_2 _detectedcomponents
          (`PrimitiveComponent.SetMaterial` _array_element_2 0 (`BlueprintMapLibrary.Map_Find` _meshmatmap _array_element_2)))
        (`KismetArrayLibrary.Array_Clear` _detectedcomponents)
        (`BlueprintMapLibrary.Map_Clear` _meshmatmap)))))

(fn `SlowMotion`
  (params (TimeAlpha :type "Float (double-precision)"))
  ;[1 1 1] Fadeout the Slow Effect
  (`GameplayStatics.SetGlobalTimeDilation` (`KismetMathLibrary.Lerp` 0.1 1.0 TimeAlpha)))

(fn `SmoothCamera`
  (bind _iscameraxfree (`self.IsCameraXFree`))
  (bind _iscamerayfree (`self.IsCameraYFree`))
  (bind (_returnvalue_x _returnvalue_y _returnvalue_z) (`KismetMathLibrary.BreakVector` (`SceneComponent.K2_GetComponentLocation` (`self.SpringArm`))))
  (bind (_returnvalue_x_2 _returnvalue_y_2 _returnvalue_z_2) (`KismetMathLibrary.BreakVector` (`KismetMathLibrary.VLerp` (`KismetMathLibrary.MakeVector` _returnvalue_x _returnvalue_y _returnvalue_z) (+ (`self.K2_GetActorLocation`) (`self.GetVelocity`)) (* (`GameplayStatics.GetWorldDeltaSeconds`) (`self.SmoothCameraSpeed`)))))
  (if (`self.SmoothCameraExtend`)
    ;[1 1 1] Check the directions
    (if (and _iscameraxfree _iscamerayfree)
      ;[1 1 1] The Camera will extend forward (Remember to adjust camera speed)
      (`SceneComponent.K2_SetWorldLocation` (`self.SpringArm`) (`KismetMathLibrary.MakeVector` _returnvalue_x_2 _returnvalue_y_2 _returnvalue_z_2) false false)
      (elif _iscameraxfree
        (`SceneComponent.K2_SetWorldLocation` (`self.SpringArm`) (`KismetMathLibrary.MakeVector` _returnvalue_x_2 _returnvalue_y _returnvalue_z_2) false false)
        (elif _iscamerayfree
          (`SceneComponent.K2_SetWorldLocation` (`self.SpringArm`) (`KismetMathLibrary.MakeVector` _returnvalue_x _returnvalue_y_2 _returnvalue_z_2) false false))))
    (set `self.IsCameraXFree` true)
    (set `self.IsCameraYFree` true)
    ;[1 1 1] Hard reset the camera if the player and the camera is too far apart
    (if (>= (`KismetMathLibrary.Vector_Distance` (`self.K2_GetActorLocation`) (`SceneComponent.K2_GetComponentLocation` (`self.SpringArm`))) 200.0)
      ;[1 1 1] The Camera will follow player (Remember to adjust camera speed)
      (`SceneComponent.K2_SetWorldLocation` (`self.SpringArm`) (`KismetMathLibrary.VLerp` (`SceneComponent.K2_GetComponentLocation` (`self.SpringArm`)) (`self.K2_GetActorLocation`) (* (`GameplayStatics.GetWorldDeltaSeconds`) (* (`self.SmoothCameraSpeed`) 2.0))) false false :!label _label))
    (else
      (goto _label))))

(fn `ThrowObject`
  (bind _staticmesh (`/Game/Assets/Blueprints/Bohan/GrabAndThrowObject/BP_GrabItem.StaticMesh` (`self.HoldingItem`)))
  ;[1 1 1] Unparent Object
  (if (`self.IsHoldingItem`)
    (`self.K2_DetachFromActor` (`self.HoldingItem`) "KeepRelative" "KeepWorld" "KeepRelative")
    (`self.K2_SetActorLocation` (`self.HoldingItem`) (`SceneComponent.K2_GetComponentLocation` (`self.ThrowDirection`)) false true)
    (`PrimitiveComponent.SetSimulatePhysics` _staticmesh true)
    (`PrimitiveComponent.SetCollisionEnabled` _staticmesh "QueryAndPhysics")
    (if (`/Game/Assets/Blueprints/Bohan/GrabAndThrowObject/BP_GrabItem.IsLargeObject` (`self.HoldingItem`))
      ;[1 1 1] Throw The Object Out With Power
      (`PrimitiveComponent.AddForce` (`/Game/Assets/Blueprints/Bohan/GrabAndThrowObject/BP_GrabItem.StaticMesh` (`self.HoldingItem`)) (* (`SceneComponent.GetForwardVector` (`self.ThrowDirection`)) (`self.SpinPower`)) "None" true)
      (set `self.IsHoldingItem` false)
      (else
        ;[1 1 1] Throw The Object Out With Power
        (`PrimitiveComponent.AddForce` (`/Game/Assets/Blueprints/Bohan/GrabAndThrowObject/BP_GrabItem.StaticMesh` (`self.HoldingItem`)) (* (`SceneComponent.GetForwardVector` (`self.ThrowDirection`)) (`self.ThrowPower`)) "None" true)
        (set `self.IsHoldingItem` false)))
    ;[1 1 1] Add Random Angular Velocity
    (`PrimitiveComponent.AddAngularImpulseInDegrees` (`/Game/Assets/Blueprints/Bohan/GrabAndThrowObject/BP_GrabItem.StaticMesh` (`self.HoldingItem`)) (`KismetMathLibrary.MakeVector` (`KismetMathLibrary.RandomFloatInRange` 0.0 500.0) (`KismetMathLibrary.RandomFloatInRange` 0.0 500.0) (`KismetMathLibrary.RandomFloatInRange` 0.0 500.0)) "None" true)
    (if (`/Game/Assets/Blueprints/Bohan/GrabAndThrowObject/BP_GrabItem.IsLargeObject` (`self.HoldingItem`))
      (`self.K2_AddActorWorldOffset` (* (`self.GetActorForwardVector`) -100.0) true)
      (set `self.SpinPower` 20000.0)
      (set `CharacterMovementComponent.MaxWalkSpeed` 600.0 (`self.CharacterMovement`))
      (set `CharacterMovementComponent.JumpZVelocity` 600.0 (`self.CharacterMovement`))
      (set `self.SpinSpeed` 0.0)
      (set `self.bIsHolding` false)
      (`KismetSystemLibrary.PrintString` "Throw"))))

(fn `UserConstructionScript`
  (bind _mesh (`self.Mesh`))
  ;[1 1 1] Attach Hand Collision To Mesh Sockets
  (`SceneComponent.K2_AttachToComponent` (`self.LeftHandCollision`) _mesh "hand_lSocket" "KeepRelative" "KeepRelative" "KeepRelative" true)
  (`SceneComponent.K2_AttachToComponent` (`self.RightHandCollision`) _mesh "hand_rSocket" "KeepRelative" "KeepRelative" "KeepRelative" true)
  (`SceneComponent.K2_AttachToComponent` (`self.RightFootCollision`) _mesh "foot_rSocket" "KeepRelative" "KeepRelative" "KeepRelative" true)
  ;[1 1 1] Setup initial camera position (camera is using absolute location)
  (`SceneComponent.K2_SetWorldLocation` (`self.SpringArm`) (`self.K2_GetActorLocation`) false true)
  (if (`self.ShowCameraLineCheck`)
    (set `self.TraceDebug` "ForDuration")
    (else
      (set `self.TraceDebug` "None"))))