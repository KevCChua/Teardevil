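; Game Instance Blueprint that holds the game's Score value.
; Three events for adding, clearing and setting the score each forward to a matching function.
; These functions update the Score variable, and AddScore also prints a score value as a string.
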(event `AddScoreEvent`
  (params (Score :type Integer))
  ;[1 0.4844 0.4844] Score Events
  (`self.AddScore` Score))

(event `ClearScoreEvent`
  ;[1 0.4844 0.4844] Score Events
  (`self.ClearScore`))

(event `SetScoreEvent`
  (params (Score :type Integer))
  ;[1 0.4844 0.4844] Score Events
  (`self.SetScore` Score))

(fn `AddScore`
  (params (score :type Integer))
  (bind _output_get (set `self.Score` (+ (`self.Score`) score)))
  (`KismetSystemLibrary.PrintString` (`KismetStringLibrary.Conv_IntToString` _output_get) true true (struct :`G` 0.66 :`B` 1.0 :`A` 1.0) 5.0))

(fn `ClearScore`
  (set `self.Score` 0))

(fn `SetScore`
  (params (NewScore :type Integer))
  (set `self.Score` NewScore))